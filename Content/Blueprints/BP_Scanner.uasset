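; BP_Scanner is a scanner Blueprint that signals when evidence is inside its scan area.
; Every Tick it checks the actors overlapping ScanArea, looking for an EvidenceBase.
; A Detecting flag limits material changes to state transitions, switching StaticMesh to ArrowMaterial on detection and back to BasicAsset01 when none is found.
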(event EventBeginPlay)

(event Collision|EventActorBeginOverlap
  (params (OtherActor :type Actor%20Object%20Reference)))

(event EventTick
  (params (DeltaSeconds :type Float%20%28single-precision%29))
  (bind _array_element (Utilities|Array|ForEachLoopwithBreak (Collision|GetOverlappingActors (Variables|Default|GetScanArea) 0 :!class /Script/Engine.PrimitiveComponent) :!label _label)
    (:LoopBody
      (Variables|Default|SetBroken false)
      (Utilities|Casting|CastToEvidenceBase _array_element)
      (if (Variables|Default|GetDetecting)
        _
        (else
          (Variables|Default|SetDetecting true)
          (Rendering|Material|SetMaterial (Variables|Default|GetStaticMesh) 0 "/Engine/VREditor/UI/ArrowMaterial.ArrowMaterial")))
      (Variables|Default|SetBroken true)
      (goto _label Break))
    (:Completed
      (if (not (Variables|Default|GetBroken))
        (if (Variables|Default|GetDetecting)
          (Variables|Default|SetDetecting false)
          (Rendering|Material|SetMaterial (Variables|Default|GetStaticMesh) 0 "/Engine/MapTemplates/Materials/BasicAsset01.BasicAsset01"))))))

(fn ConstructionScript)