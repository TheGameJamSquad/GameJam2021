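; BP_ExitDoor is an exit trigger that opens the exit-loop screen when the player reaches it carrying evidence.
; On ExitCollider overlap, it scans overlapping actors for a BP_MyPlayer whose handled actor is an EvidenceBase.
; It then disables that player's movement, creates W_ExitLoop with a reference to the player, and switches player controller 0 to UI-only input with a visible cursor.
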(event OnComponentBeginOverlap(ExitCollider)
  (params (OverlappedComponent :type Primitive%20Component%20Object%20Reference) (OtherActor :type Actor%20Object%20Reference) (OtherComp :type Primitive%20Component%20Object%20Reference) (OtherBodyIndex :type Integer) (bFromSweep :type Boolean) (SweepResult :type Hit%20Result%20Structure%20%28by%20ref%29))
  (bind _returnvalue (Game|GetPlayerController 0))
  (for _array_element (Collision|GetOverlappingActors (Variables|Default|GetExitCollider) 0 :!class /Script/Engine.PrimitiveComponent)
    (bind _asbp_my_player (Utilities|Casting|CastToBP_MyPlayer _array_element))
    (Variables|Default|SetPlayer _asbp_my_player)
    (Utilities|Casting|CastToEvidenceBase (Class|MyPlayer|GetHandledActor _asbp_my_player))
    (Pawn|Components|CharacterMovement|DisableMovement (Variables|/Script/Engine.Character|GetCharacterMovement (Variables|Default|GetPlayer)))
    (Utilities|FlowControl|Sequence
      (:then_0
        (bind _returnvalue_2 (UserInterface|CreateWidget "/Game/Blueprints/Widgets/W_ExitLoop.W_ExitLoop_C" _returnvalue))
        (Variables|/Game/Blueprints/Widgets/W_ExitLoop.W_ExitLoop_C|SetPlayer _returnvalue_2 (Variables|Default|GetPlayer))
        (UserInterface|Viewport|AddtoViewport _returnvalue_2 0))
      (:then_1
        (Variables|/Script/Engine.PlayerController|SetbShowMouseCursor _returnvalue true)
        (Input|SetInputModeUIOnly _returnvalue _returnvalue_2 "DoNotLock")))))

(event EventBeginPlay)

(event Collision|EventActorBeginOverlap
  (params (OtherActor :type Actor%20Object%20Reference)))

(event EventTick
  (params (DeltaSeconds :type Float%20%28single-precision%29)))

(fn ConstructionScript)