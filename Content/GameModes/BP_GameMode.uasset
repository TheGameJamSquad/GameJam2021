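; BP_GameMode is the game mode for an evidence game, holding the time limit and the evidence that counts as final.
; BeginPlay and RestoreValues reset GameTimeLeft from GameTimeInSeconds, while StartGameTimer is empty and nothing here counts down.
; ChooseFinalEvidence picks a random RealEvidence actor from the level.
; CheckFinalEvidence matches the player's held EvidenceBase to it by comparing mesh mass rather than actor identity.
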(event EventBeginPlay
  (CallFunction|SetGameTimer))

(event EventTick
  (params (DeltaSeconds :type Float%20%28single-precision%29)))

(fn ConstructionScript)

(fn StartGameTimer)

(fn SetGameTimer
  (Variables|Default|SetGameTimeLeft (Math|Conversions|ToFloat(Integer) (Variables|Default|GetGameTimeInSeconds))))

(fn RestoreValues
  (CallFunction|SetGameTimer))

(fn ChooseFinalEvidence
  (bind _outactors (Actor|GetAllActorsOfClass "/Game/Blueprints/Test/RealEvidence.RealEvidence_C"))
  (Variables|Default|SetFinalEvidence (Utilities|Array|Get(acopy) _outactors (Math|Random|RandomInteger (Utilities|Array|Length _outactors)))))

(fn CheckFinalEvidence
  (bind _playeritem (CallFunction|GetItemHeldbyPlayer))
  (return (== (Physics|GetMass (Variables|/Script/UnrealGameJam.EvidenceBase|GetMeshComponent _playeritem)) (Physics|GetMass (Variables|/Script/UnrealGameJam.EvidenceBase|GetMeshComponent (Variables|Default|GetFinalEvidence))))))

(fn GetItemHeldbyPlayer
  (bind _asbp_my_player (Utilities|Casting|CastToBP_MyPlayer (Game|Player|GetPlayerPawn 0)))
  (bind _asevidence_base (Utilities|Casting|CastToEvidenceBase (Class|MyPlayer|GetHandledActor _asbp_my_player)))
  (return _asevidence_base))